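; InteractiveBP is a test interactive object whose Type enum picks its mesh from an array, with a trigger scaled in the construction script.
; When a BP_PickupCube2 actor begins overlapping it, ItemMesh is hidden.
; An older key/lock path that matches a PickupBP's Type to per-type unlock messages is disconnected and never runs, including the event that destroys the pickup.
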(event `self.ReceiveActorBeginOverlap`
  (params (OtherActor :type "Actor Object Reference"))
  (cast `/Game/VirtualRealityBP/Blueprints/BP_PickupCube2` OtherActor)
  (`SceneComponent.SetVisibility` (`self.ItemMesh`) false false))

(event `0Key1`
  (`KismetSystemLibrary.PrintString` "Key 1 has unlocked this special bulletin message")
  (`self.K2_DestroyActor` (`self.PickupRef`)))

(event `1Key2`
  (`KismetSystemLibrary.PrintString` "Key 2 has unlocked this special bulletin message"))

(event `2Key3`
  (`KismetSystemLibrary.PrintString` "Key 3 has unlocked this special bulletin message"))

(event `3Safe1`
  (`KismetSystemLibrary.PrintString` "Pretend Key has unlocked this special bulletin message"))

(fn `UserConstructionScript`
  (`|ExecutionSequence`
    (:`then_0`
      (`SceneComponent.SetWorldScale3D` (`self.Trigger`) (`KismetMathLibrary.MakeVector` (`self.TriggerX`) (`self.TriggerY`) (`self.TriggerZ`))))
    (:`then_1`
      (`StaticMeshComponent.SetStaticMesh` (`self.ItemMesh`) (`KismetArrayLibrary.Array_Get` (`self.MeshArray`) (`KismetMathLibrary.Conv_ByteToInt` (`self.Type`)))))))